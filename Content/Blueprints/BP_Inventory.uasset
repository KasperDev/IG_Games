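; Inventory Blueprint that stores items as data-table row references with amounts in a fixed slot array and creates the main inventory widget on BeginPlay.
; AddItemInTable fills free stacks, then empty slots, recursing on overflow; the older AddItem is an empty stub.
; Swap, split and remove refresh affected slot widgets; removal also spawns a BP_MasterItem near the character.
; Equip sends matching item types to the quick-slot icon and character's EquipWeapons.
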(event Custom|UpdateSlotAtIndex
  (params (Index :type Integer))
  (Default|UpdateSlots (Utilities|Array|Get(acopy) (Variables|/Game/Blueprints/Witgets/W_Inventory.W_Inventory_C|GetSlotsWitgets (Variables|Default|GetW%20Inventory)) Index)))

(event Custom|UseItemAtIndex
  (params (Index :type Integer)))

(event EventBeginPlay
  (Utilities|Array|Resize (Variables|Default|GetSlots) (Variables|Default|GetAmountOfSlotz))
  (bind _returnvalue (UserInterface|CreateWidget "/Game/Blueprints/Witgets/W_Main.W_Main_C" 0 self (Variables|Default|GetSlot%20Per%20Row)))
  (bind _output_get (Variables|Default|SetMainWitget _returnvalue))
  (Variables|Default|SetW%20Inventory (Variables|/Game/Blueprints/Witgets/W_Main.W_Main_C|GetW_Inventory _output_get))
  (UserInterface|Viewport|AddtoViewport (Variables|Default|GetMainWitget) 0))

(fn ConstructionScript)

(fn IsSlotEmpty?
  (params (Index :type Integer))
  (return (not (Utilities|IsValid (.DataTable (Utilities|Struct|BreakDataTableRowHandle (.ItemDataTable (Utilities|Struct|BreakStruct_InventorySlot (Utilities|Array|Get(acopy) (Variables|Default|GetSlots) Index)))))))))

(fn GetItemInfoatIndex
  (params (Index :type Integer))
  (bind _slots (Variables|Default|GetSlots))
  (bind _output (Utilities|Array|Get(acopy) _slots Index))
  (bind (_itemdatatable _amount) (Utilities|Struct|BreakStruct_InventorySlot _output))
  (if (Utilities|IsValid (.DataTable (Utilities|Struct|BreakDataTableRowHandle _itemdatatable)))
    (bind _asmasteritem (CallFunction|GetItemInfo _itemdatatable))
    (return false (.baseiteminfo _asmasteritem) _amount)
    (else
      (return true "" 0))))

(fn SearchEmptySlot
  (bind (_array_element _array_index) (Utilities|Array|ForEachLoopwithBreak (Variables|Default|GetSlots) :!label _label)
    (:LoopBody
      (if (not (Utilities|IsValid (.datatable (.ItemDataTable (Utilities|Struct|BreakStruct_InventorySlot _array_element)))))
        (LocalVariables|SetLocalBool true)
        (LocalVariables|SetLocalIndex _array_index)
        (goto _label Break)))
    (:Completed
      (return (LocalVariables|GetLocalBool) (LocalVariables|GetLocalIndex)))))

(fn SearchFreeStack
  (params (ItemDataTable :type Data%20Table%20Row%20Handle%20Structure))
  (bind (_array_element _array_index) (Utilities|Array|ForEachLoopwithBreak (Variables|Default|GetSlots) :!label _label)
    (:LoopBody
      (if (Utilities|IsValid (.datatable (.ItemDataTable (Utilities|Struct|BreakStruct_InventorySlot _array_element))))
        (if (and (Utilities|Name|Equal(Name) (.rowname (.ItemDataTable (Utilities|Struct|BreakStruct_InventorySlot _array_element))) (.RowName (Utilities|Struct|BreakDataTableRowHandle ItemDataTable))) (< (.Amount (Utilities|Struct|BreakStruct_InventorySlot _array_element)) (Variables|Default|GetMaxStackSize)))
          (LocalVariables|SetLocalBool true)
          (LocalVariables|SetLocalIndex _array_index)
          (goto _label Break))))
    (:Completed
      (return (LocalVariables|GetLocalBool) (LocalVariables|GetLocalIndex)))))

(fn AddItem
  (params (ItemClass :type BP%20Master%20Item%20Class%20Reference) (Amount :type Integer) (ItemDataTable :type Data%20Table%20Row%20Handle%20Structure)))

(fn GetAmountatIndex
  (params (Index :type Integer))
  (return (.Amount (Utilities|Struct|BreakStruct_InventorySlot (Utilities|Array|Get(acopy) (Variables|Default|GetSlots) Index)))))

(fn AddIteminTable
  (params (ItemDataTable :type Data%20Table%20Row%20Handle%20Structure) (Amaunt :type Integer))
  (LocalVariables|SetLocalItemDataTable ItemDataTable)
  (LocalVariables|SetLocalAmaunt Amaunt)
  (bind _asmasteritem (CallFunction|GetItemInfo (LocalVariables|GetLocalItemDataTable)))
  (if (.CanByStack? (Utilities|Struct|BreakStruct_BaseItemInfo (.BaseItemInfo (Utilities|Struct|BreakStruct_MasterItem _asmasteritem))))
    (bind (_success _index) (CallFunction|SearchFreeStack (LocalVariables|GetLocalItemDataTable)))
    (if _success
      (LocalVariables|SetLocalFoundIndex _index)
      (if (> (+ (.amount (Utilities|Array|Get(acopy) (Variables|Default|GetSlots) (LocalVariables|GetLocalFoundIndex))) (LocalVariables|GetLocalAmaunt)) (Variables|Default|GetMaxStackSize))
        (LocalVariables|SetLocalAmaunt (- (+ (.amount (Utilities|Array|Get(acopy) (Variables|Default|GetSlots) (LocalVariables|GetLocalFoundIndex))) (LocalVariables|GetLocalAmaunt)) (LocalVariables|GetLocalAmaunt)))
        (Utilities|Array|SetArrayElem (Variables|Default|GetSlots) (LocalVariables|GetLocalFoundIndex) (Utilities|Struct|MakeStruct_InventorySlot (LocalVariables|GetLocalItemDataTable) (Variables|Default|GetMaxStackSize)))
        (CallFunction|UpdateSlotatIndex (LocalVariables|GetLocalFoundIndex))
        (bind _rest (CallFunction|AddIteminTable (LocalVariables|GetLocalItemDataTable) (LocalVariables|GetLocalAmaunt)))
        (return true _rest)
        (else
          ;[1 1 1] Comment
          (Utilities|Array|SetArrayElem (Variables|Default|GetSlots) (LocalVariables|GetLocalFoundIndex) (Utilities|Struct|MakeStruct_InventorySlot (LocalVariables|GetLocalItemDataTable) (+ (.amount (Utilities|Array|Get(acopy) (Variables|Default|GetSlots) (LocalVariables|GetLocalFoundIndex))) (LocalVariables|GetLocalAmaunt))))
          (CallFunction|UpdateSlotatIndex (LocalVariables|GetLocalFoundIndex))
          (return true 0)))
      (else
        (bind (_success_2 _index_2) (CallFunction|SearchEmptySlot))
        (if _success_2
          (bind _output_get (LocalVariables|SetLocalFoundIndex _index_2))
          (if (> (LocalVariables|GetLocalAmaunt) (Variables|Default|GetMaxStackSize))
            (Utilities|Array|SetArrayElem (Variables|Default|GetSlots) _output_get (Utilities|Struct|MakeStruct_InventorySlot (LocalVariables|GetLocalItemDataTable) (Variables|Default|GetMaxStackSize)))
            (CallFunction|UpdateSlotatIndex (LocalVariables|GetLocalFoundIndex))
            (bind _rest_2 (CallFunction|AddIteminTable (LocalVariables|GetLocalItemDataTable) (- (LocalVariables|GetLocalAmaunt) (Variables|Default|GetMaxStackSize))))
            (return true _rest_2)
            (else
              (Utilities|Array|SetArrayElem (Variables|Default|GetSlots) (LocalVariables|GetLocalFoundIndex) (Utilities|Struct|MakeStruct_InventorySlot (LocalVariables|GetLocalItemDataTable) (LocalVariables|GetLocalAmaunt)))
              (CallFunction|UpdateSlotatIndex (LocalVariables|GetLocalFoundIndex))
              (return true 0)))
          (else
            (return false (LocalVariables|GetLocalAmaunt))))))
    (else
      (bind (_success_3 _index_3) (CallFunction|SearchEmptySlot))
      (if _success_3
        (bind _output_get_2 (LocalVariables|SetLocalFoundIndex _index_3))
        (Utilities|Array|SetArrayElem (Variables|Default|GetSlots) _output_get_2 (Utilities|Struct|MakeStruct_InventorySlot (LocalVariables|GetLocalItemDataTable) 1))
        (CallFunction|UpdateSlotatIndex (LocalVariables|GetLocalFoundIndex))
        (if (> (LocalVariables|GetLocalAmaunt) 1)
          (bind _rest_3 (CallFunction|AddIteminTable (LocalVariables|GetLocalItemDataTable) (- (LocalVariables|GetLocalAmaunt) 1)))
          (return true _rest_3)
          (else
            (return true 0)))
        (else
          (return false (LocalVariables|GetLocalAmaunt)))))))

(fn GetIinfo
  (params (Index :type Integer))
  (bind _slots (Variables|Default|GetSlots))
  (bind _output (Utilities|Array|Get(acopy) _slots Index))
  (bind _itemdatatable (Utilities|Struct|BreakStruct_InventorySlot _output))
  (if (Utilities|IsValid (.DataTable (Utilities|Struct|BreakDataTableRowHandle _itemdatatable)))
    (return false _itemdatatable)
    (else
      (return true ""))))

(fn Equip
  (params (index :type Integer))
  (bind _mainwitget (Variables|Default|GetMainWitget))
  (bind _w_quickslot (Variables|/Game/Blueprints/Witgets/W_Main.W_Main_C|GetW_QuickSlot _mainwitget))
  (bind _slotimages_1 (Variables|/Game/Blueprints/Witgets/W_QuickSlot.W_QuickSlot_C|GetSlotimages_1 _w_quickslot))
  (bind _output_get (LocalVariables|SetLocalIndex index))
  (bind _iteminfo (CallFunction|GetIinfo _output_get))
  (bind _asmasteritem (CallFunction|GetItemInfo _iteminfo))
  (LocalVariables|SetLocalItemInfo _iteminfo)
  (if (Utilities|Enum|Equal(Enum) (.baseitemtype (.BaseItemInfo (Utilities|Struct|BreakStruct_MasterItem _asmasteritem))) "NewEnumerator1")
    (Appearance|SetBrushfromTexture _slotimages_1 (.icon (.BaseItemInfo (Utilities|Struct|BreakStruct_MasterItem _asmasteritem))) false)
    (Widget|SetVisibility _slotimages_1 "HitTestInvisible")
    (Default|EquipWeapons (Variables|Default|GetCharactersRef) (LocalVariables|GetLocalItemInfo))
    (else
      (Development|PrintString "NOT EQIP")
      (return))))

(fn RemoveItematIndex
  (params (LocalIndex :type Integer) (LocalAmount :type Integer))
  (bind _slots (Variables|Default|GetSlots))
  (bind _charactersref (Variables|Default|GetCharactersRef))
  (bind _mesh (Variables|/Script/Engine.Character|GetMesh _charactersref))
  (bind _returnvalue (Transformation|GetWorldLocation _mesh))
  (bind _returnvalue_2 (+ _returnvalue "100.000000, 0,50.000000"))
  (bind _output_get (LocalVariables|SetLocal_Index LocalIndex))
  (LocalVariables|SetLocal_amount LocalAmount)
  (LocalVariables|SetLocalDT (Utilities|Array|Get(acopy) (Variables|Default|GetSlots) _output_get))
  (if (and (not (CallFunction|IsSlotEmpty? (LocalVariables|GetLocal_Index))) (> (LocalVariables|GetLocal_amount) 0))
    (if (>= (LocalVariables|GetLocal_amount) (CallFunction|GetAmountatIndex (LocalVariables|GetLocal_Index)))
      (Utilities|Array|SetArrayElem (Variables|Default|GetSlots) (LocalVariables|GetLocal_Index) (Utilities|Struct|MakeStruct_InventorySlot "(DataTable=None,RowName=\"\")" 0))
      (CallFunction|UpdateSlotatIndex (LocalVariables|GetLocal_Index))
      (Game|SpawnActorfromClass "/Game/Blueprints/BP_MasterItem.BP_MasterItem_C" (Math|Transform|MakeTransform _returnvalue_2 "0, 0, 0" "1,1,1") "AlwaysSpawn" 0 (.itemdatatable (LocalVariables|GetLocalDT)) 1 0)
      (return true)
      (else
        (Utilities|Array|SetArrayElem _slots (LocalVariables|GetLocal_Index) (Utilities|Struct|MakeStruct_InventorySlot (.itemdatatable (Utilities|Array|Get(acopy) _slots (LocalVariables|GetLocal_Index))) (- (.amount (Utilities|Array|Get(acopy) _slots (LocalVariables|GetLocal_Index))) (LocalVariables|GetLocal_amount))))
        (CallFunction|UpdateSlotatIndex (LocalVariables|GetLocal_Index))
        (Game|SpawnActorfromClass "/Game/Blueprints/BP_MasterItem.BP_MasterItem_C" (Math|Transform|MakeTransform _returnvalue_2 "0, 0, 0" "1,1,1") "AlwaysSpawn" 0 (.itemdatatable (LocalVariables|GetLocalDT)) 1 0)
        (return true)))
    (else
      (return false))))

(fn SwapSlots
  (params (Index1 :type Integer) (Index2 :type Integer))
  (bind _slots (Variables|Default|GetSlots))
  (bind _slots_2 (Variables|Default|GetSlots))
  (bind _returnvalue (Utilities|Array|LastIndex _slots))
  (LocalVariables|SetLocalIndex1 Index1)
  (LocalVariables|SetLocalIndex2 Index2)
  (if (or (> (LocalVariables|GetLocalIndex1) _returnvalue) (> (LocalVariables|GetLocalIndex2) _returnvalue))
    (return false)
    (else
      (LocalVariables|SetLocalSlot_2 (Utilities|Array|Get(acopy) (Variables|Default|GetSlots) (LocalVariables|GetLocalIndex2)))
      (Utilities|Array|SetArrayElem _slots_2 (LocalVariables|GetLocalIndex2) (Utilities|Array|Get(acopy) _slots_2 (LocalVariables|GetLocalIndex1)))
      (Utilities|Array|SetArrayElem (Variables|Default|GetSlots) (LocalVariables|GetLocalIndex1) (LocalVariables|GetLocalSlot_2))
      (CallFunction|UpdateSlotatIndex (LocalVariables|GetLocalIndex1))
      (CallFunction|UpdateSlotatIndex (LocalVariables|GetLocalIndex2))
      (return true))))

(fn SplitStack
  (params (StackIndex :type Integer) (Amount :type Integer))
  (bind _slots (Variables|Default|GetSlots))
  (bind _slots_2 (Variables|Default|GetSlots))
  (LocalVariables|SetLocalStackIndex StackIndex)
  (LocalVariables|SetLocalAmount Amount)
  (if (CallFunction|IsSlotEmpty? (LocalVariables|GetLocalStackIndex))
    (return false)
    (elif (and (.canbystack? (.ItemInfo (CallFunction|GetItemInfoatIndex (LocalVariables|GetLocalStackIndex)))) (> (.Amount (CallFunction|GetItemInfoatIndex (LocalVariables|GetLocalStackIndex))) (LocalVariables|GetLocalAmount)))
      (bind (_success _index) (CallFunction|SearchEmptySlot))
      (if _success
        (LocalVariables|SetLocalFoundIndex _index)
        (Utilities|Array|SetArrayElem _slots_2 (LocalVariables|GetLocalStackIndex) (Utilities|Struct|MakeStruct_InventorySlot (.itemdatatable (Utilities|Array|Get(acopy) _slots_2 (LocalVariables|GetLocalStackIndex))) (- (.amount (Utilities|Array|Get(acopy) _slots_2 (LocalVariables|GetLocalStackIndex))) (LocalVariables|GetLocalAmount))))
        (Utilities|Array|SetArrayElem _slots (LocalVariables|GetLocalFoundIndex) (Utilities|Struct|MakeStruct_InventorySlot (.itemdatatable (Utilities|Array|Get(acopy) _slots (LocalVariables|GetLocalStackIndex))) (LocalVariables|GetLocalAmount)))
        (CallFunction|UpdateSlotatIndex (LocalVariables|GetLocalStackIndex))
        (CallFunction|UpdateSlotatIndex (LocalVariables|GetLocalFoundIndex))
        (return true)
        (else
          (return false)))
      (else
        (return false)))))