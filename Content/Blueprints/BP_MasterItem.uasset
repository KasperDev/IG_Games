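; Master world item actor that represents a data-table item as a physics object players can pick up.
; On BeginPlay it resolves ConstructInfo from a valid MasterItemInfo or the ItemDataTable lookup, then applies its skeletal mesh, falling back to static.
; PickUp adds the Amount to an Inventory, keeping any remainder or destroying the actor.
; GetInfoWitget swaps the HUD crosshair for an item-name prompt; the delayed restore is unwired.
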(event EventBeginPlay
  (CallFunction|UpdateItemInfo)
  (CallFunction|UpdateItemMesh))

(event EventPickUp
  (params (Inventory :type BP%20Inventory%20Object%20Reference))
  (Utilities|IsValid Inventory
    (:Is%20Valid
      (bind (_success _rest) (Default|AddIteminTable Inventory (Variables|Default|GetItemDataTable) (Variables|Default|GetAmount)))
      (if _success
        (if (> _rest 0)
          (Variables|Default|SetAmount _rest)
          (else
            (Actor|DestroyActor)))))))

(event EventGetInfoWitget
  (params (W_Main :type W%20Main%20Object%20Reference))
  (bind _view_ (CallFunction|GetWitgetInfo W_Main true))
  (if _view_
    _))

(fn ConstructionScript)

(fn AddAttachment
  (params (Mesh :type Skeletal%20Mesh%20Object%20Reference)))

(fn UpdateItemMesh
  (bind _constructinfo (Variables|Default|GetConstructInfo))
  (bind _staticmesh (Variables|Default|GetStaticMesh))
  (bind _roootskeletalmesh (Variables|Default|GetRoootSkeletalMesh))
  (bind _baseiteminfo (Utilities|Struct|BreakStruct_MasterItem _constructinfo))
  (bind (_baseitemtype _name _description _icon _skeletalmesh _staticmesh_2 _scale) (Utilities|Struct|BreakStruct_BaseItemInfo _baseiteminfo))
  (bind _returnvalue (> _scale 0.0))
  (if (Utilities|IsValid _skeletalmesh)
    (Class|SkinnedMeshComponent|SetSkeletalMesh _roootskeletalmesh _skeletalmesh true)
    (Physics|SetSimulatePhysics _roootskeletalmesh true)
    (if _returnvalue
      (Class|PrimitiveComponent|SetMassScale _roootskeletalmesh "None" _scale))
    (else
      (Components|StaticMesh|SetStaticMesh _staticmesh _staticmesh_2)
      (Physics|SetSimulatePhysics _staticmesh true)
      (if _returnvalue
        (Class|PrimitiveComponent|SetMassScale _staticmesh "None" 1.0))))
  (return))

(fn UpdateItemInfo
  (bind _masteriteminfo (Variables|Default|GetMasterItemInfo))
  (bind _datatabletouse (Utilities|Struct|BreakStruct_MasterItem _masteriteminfo))
  (bind _asmasteritem (CallFunction|GetItemInfo (Variables|Default|GetItemDataTable)))
  (Variables|Default|SetConstructInfo (select (and (Utilities|IsValid (.datatable _datatabletouse)) (Utilities|Name|NotEqual(Name) (.rowname _datatabletouse) "None")) (Variables|Default|GetMasterItemInfo) _asmasteritem)))

(fn OnRepItemDataTable)

(fn RemoveAttachment
  (bind _basesmcomponent (Variables|Default|GetBaseSMComponent))
  (bind _basestaticmeshcomponent (Variables|Default|GetBaseStaticMeshComponent))
  (Utilities|IsValid _basesmcomponent
    (:Is%20Valid
      (Components|DestroyComponent _basesmcomponent))
    (:Is%20Not%20Valid
      _))
  (Utilities|IsValid _basestaticmeshcomponent
    (:Is%20Valid
      (Components|DestroyComponent _basestaticmeshcomponent))))

(fn OnRepAmount)

(fn GetWitgetInfo
  (params (W_Main :type W%20Main%20Object%20Reference) (View :type Boolean))
  (LocalVariables|SetLocal_CrossHair (Variables|/Game/Blueprints/Witgets/W_Main.W_Main_C|GetCrossHair W_Main))
  (LocalVariables|SetLocal_UserInterakt (Variables|/Game/Blueprints/Witgets/W_Main.W_Main_C|GetUserInterakt W_Main))
  (if View
    (Widget|SetVisibility (LocalVariables|GetLocal_CrossHair) "Hidden")
    (Widget|SetVisibility (LocalVariables|GetLocal_UserInterakt) "Visible")
    (Rendering|Components|TextRender|SetText (Variables|/Game/Blueprints/Witgets/UserInterakt.UserInterakt_C|GetItemName (LocalVariables|GetLocal_UserInterakt)) (.name (.baseiteminfo (Variables|Default|GetConstructInfo))))
    (return true)
    (else
      (Widget|SetVisibility (LocalVariables|GetLocal_CrossHair) "Visible")
      (Widget|SetVisibility (LocalVariables|GetLocal_UserInterakt) "Hidden")
      (Rendering|Components|TextRender|SetText (Variables|/Game/Blueprints/Witgets/UserInterakt.UserInterakt_C|GetItemName (LocalVariables|GetLocal_UserInterakt)) "")
      (return false))))