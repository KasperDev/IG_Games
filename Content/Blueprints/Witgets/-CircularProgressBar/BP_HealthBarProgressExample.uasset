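; Example Blueprint that demonstrates the adjustable circular progress bar widget as an animated health bar.
; On BeginPlay it creates the widget, adds it to the viewport and starts a timeline that drives the progress of four bars with the same value.
; A boolean flips the timeline between forward and reverse playback each time it finishes, so the bars animate back and forth endlessly.
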(event Custom|HealthDown
  (bind _healthwidget (Variables|Default|GetHealthWidget))
  (Variables|Default|SetIsHealthDown true)
  (bind _1_0 (Timeline|Timeline_0 PlayFromStart)
    (:Update
      (Default|SetProgress _healthwidget _1_0)
      (Default|SetProgress _healthwidget _1_0 1)
      (Default|SetProgress _healthwidget _1_0 2)
      (Default|SetProgress _healthwidget _1_0 3))
    (:Finished
      (if (Variables|Default|GetIsHealthDown)
        (CallFunction|HealthUp)
        (else
          (CallFunction|HealthDown))))))

(event Custom|HealthUp
  (bind _healthwidget (Variables|Default|GetHealthWidget))
  (Variables|Default|SetIsHealthDown false)
  (bind _1_0 (Timeline|Timeline_0 ReverseFromEnd)
    (:Update
      (Default|SetProgress _healthwidget _1_0)
      (Default|SetProgress _healthwidget _1_0 1)
      (Default|SetProgress _healthwidget _1_0 2)
      (Default|SetProgress _healthwidget _1_0 3))
    (:Finished
      (if (Variables|Default|GetIsHealthDown)
        (CallFunction|HealthUp)
        (else
          (CallFunction|HealthDown))))))

(event EventBeginPlay
  (bind _returnvalue (UserInterface|CreateWidget "/Game/Blueprints/Witgets/-CircularProgressBar/AdjustableCircularBar_Widget.AdjustableCircularBar_Widget_C"))
  (bind _output_get (Variables|Default|SetHealthWidget _returnvalue))
  (UserInterface|Viewport|AddtoViewport _output_get 0)
  (CallFunction|HealthDown))

(fn ConstructionScript)