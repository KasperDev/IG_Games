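; Equippable weapon actor that loads its stats from item data, attaches its mesh to the character's hand socket and drives the ammo HUD.
; Automatic fire loops through a gate and retriggerable delay, playing montages and spending ammo.
; Each shot traces from the active camera to aim BP_Bullet from the muzzle, adding random negative-only spread.
; Reloading blocks new fire for a delay and refills the clip from reserve ammo.
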(event Custom|StartFire
  (if (Variables|Default|GetAttached?)
    (if (not (Variables|WeaponsSetting|GetIsReloading?))
      (Utilities|FlowControl|Sequence
        (:then_0
          (goto _label Open))
        (:then_1
          (Utilities|FlowControl|Gate true :!label _label
            (:Exit
              (Utilities|FlowControl|Sequence
                (:then_0
                  (Utilities|FlowControl|RetriggerableDelay (Variables|WeaponsSetting|GetFireRait))
                  (goto _label))
                (:then_1
                  (CallFunction|InfoPanelUpdate)
                  (if (> (Utilities|Struct|BreakStruct_ShootingSettings (Utilities|Struct|BreakStruct_MasterWeapon (Variables|Default|GetMasterWeaponInfo))) 0)
                    (FireAction|SpawnProjectTile)
                    (|SetData (Variables|Default|GetMasterWeaponInfo))))))))))))

(event Custom|StopFire
  (if (Variables|Default|GetAttached?)
    (Utilities|FlowControl|Gate true) ; enters at Toggle
  ))

(event Custom|FirePress
  (CallFunction|StartFire))

(event Custom|FireRelise
  (CallFunction|StopFire))

(event Custom|StartReload
  (bind _masterweaponinfo (Variables|Default|GetMasterWeaponInfo))
  (bind _shootingdata (Utilities|Struct|BreakStruct_MasterWeapon _masterweaponinfo))
  (bind (_reloaddelay _ammomax _ammocurrent _ammoinclip) (Utilities|Struct|BreakStruct_ShootingSettings _shootingdata))
  (if (not (== _ammomax 0))
    (if (not (== _ammocurrent _ammoinclip))
      (bind _output_get (Variables|WeaponsSetting|SetIsReloading? true))
      (if _output_get
        (CallFunction|StopFire)
        (CallFunction|Reload)
        (Utilities|FlowControl|Delay _reloaddelay)
        (Variables|WeaponsSetting|SetIsReloading? false)
        (Development|PrintString (Utilities|String|ToString(Float) _reloaddelay))))))

(fn ConstructionScript)

(fn UpdateItemInfo
  (params (ItemDataTable :type Data%20Table%20Row%20Handle%20Structure))
  (bind _masteriteminfo (Variables|Default|GetMasterItemInfo))
  (bind _datatabletouse (Utilities|Struct|BreakStruct_MasterItem _masteriteminfo))
  (bind _asmasteritem (CallFunction|GetItemInfo ItemDataTable))
  (bind _asmasterweapon (CallFunction|GetItemasWeapon _asmasteritem))
  (Variables|Default|SetConstructInfo _asmasteritem)
  (bind _output_get (Variables|Default|SetMasterWeaponInfo (select (and (Utilities|IsValid (.datatable _datatabletouse)) (Utilities|Name|NotEqual(Name) (.rowname _datatabletouse) "None")) (Variables|Default|GetDTWeapons) _asmasterweapon)))
  (Variables|Default|SetBase%20Weapon%20Type (.BaseWeaponType (Utilities|Struct|BreakStruct_MasterWeapon _output_get)))
  (Variables|Default|SetW%20Weapon%20Info (Variables|/Game/Blueprints/Witgets/W_Main.W_Main_C|GetW_WeaponInfo (Variables|/Game/Blueprints/BP_Inventory.BP_Inventory_C|GetMainWitget (Variables|/Game/Blueprints/Character/ThirdPersonCharacter.ThirdPersonCharacter_C|GetInventoryRef (Variables|Default|GetCharactersRef)))))
  (CallFunction|InfoPanelUpdate)
  (Widget|SetVisibility (Variables|Default|GetW%20Weapon%20Info) "Visible")
  (return))

(fn UpdateMesh
  (bind _constructinfo (Variables|Default|GetConstructInfo))
  (bind _baseiteminfo (Utilities|Struct|BreakStruct_MasterItem _constructinfo))
  (bind (_baseitemtype _name _description _icon _skeletalmesh _staticmesh _scale _canbystack_ _canbyused_ _usetxt _animclass) (Utilities|Struct|BreakStruct_BaseItemInfo _baseiteminfo))
  (Class|SkinnedMeshComponent|SetSkeletalMesh (Variables|Default|GetSkeletalMesh) _skeletalmesh true)
  (Camera|CameraUpdate)
  (if (Utilities|IsValidClass _animclass)
    (Class|SkeletalMeshComponent|SetAnimClass (Variables|Default|GetSkeletalMesh) _animclass)
    (return)
    (else
      (return))))

(fn AttachtoHand
  (bind _skeletalmesh (Variables|Default|GetSkeletalMesh))
  (if (Utilities|Enum|Equal(Enum) (.baseitemtype (.BaseItemInfo (Utilities|Struct|BreakStruct_MasterItem (Variables|Default|GetConstructInfo)))) "NewEnumerator1")
    (Transformation|AttachComponentToComponent _skeletalmesh (Variables|/Script/Engine.Character|GetMesh (Variables|Default|GetCharactersRef)) (Utilities|Select :Index (.BaseWeaponType (Utilities|Struct|BreakStruct_MasterWeapon (Variables|Default|GetMasterWeaponInfo))) :NewEnumerator0 "SKT_Weapon" :NewEnumerator1 "SKT_Weapon" :NewEnumerator2 "SKT_Shotgun" :NewEnumerator3 "SKT_Weapon" :NewEnumerator4 "SKT_Weapon") "SnapToTarget" "SnapToTarget" "SnapToTarget" true)
    (Transformation|SetRelativeLocation _skeletalmesh "0, 0, 0" false false)
    (Camera|CameraUpdate)
    (Variables|Default|SetAttached? true)))

(fn Equip
  (params (ItemDataTable :type Data%20Table%20Row%20Handle%20Structure))
  (CallFunction|UpdateItemInfo ItemDataTable)
  (CallFunction|UpdateMesh)
  (CallFunction|AttachtoHand)
  (Variables|/Game/Blueprints/Character/ThirdPersonCharacter.ThirdPersonCharacter_C|SetWeaponType (Variables|Default|GetCharactersRef) (Variables|Default|GetBase%20Weapon%20Type)))

(fn CalculateDireclion
  (bind _returnvalue (Utilities|MuzzlePosicion))
  (bind _camera (Variables|Default|GetCamera))
  (bind _charactersref (Variables|Default|GetCharactersRef))
  (bind _camera_2 (Variables|/Game/Blueprints/Character/ThirdPersonCharacter.ThirdPersonCharacter_C|GetCamera _charactersref))
  (bind _aiming (Variables|/Game/Blueprints/Character/ThirdPersonCharacter.ThirdPersonCharacter_C|GetAiming _charactersref))
  (bind _returnvalue_2 (select _aiming _camera _camera_2))
  (bind _returnvalue_3 (Transformation|GetWorldTransform _returnvalue_2))
  (bind _returnvalue_4 (|EndPoint (.rotation _returnvalue_3) (.location _returnvalue_3)))
  (bind (_outhit _returnvalue_5) (Collision|LineTraceForObjects (|StartPoint (.rotation _returnvalue_3) (.location _returnvalue_3)) _returnvalue_4 (Utilities|Array|MakeArray "ObjectTypeQuery1") false 0 "ForDuration"))
  (return _returnvalue (Math|Rotator|FindLookatRotation _returnvalue (Math|Vector|SelectVector (.ImpactPoint (Collision|BreakHitResult _outhit)) _returnvalue_4 _returnvalue_5))))

(fn CameraUpdate
  (bind _camera (Variables|Default|GetCamera))
  (bind _skeletalmesh (Variables|Default|GetSkeletalMesh))
  (Transformation|SetWorldLocation _camera (Transformation|GetSocketLocation _skeletalmesh "AimCamera") false false)
  (Transformation|SetWorldRotation _camera (Transformation|GetSocketRotation _skeletalmesh "AimCamera") false false))

(fn SpawnProjectTile
  (CallFunction|PlayMontage)
  (bind (_location _rotation) (FireAction|CalculateDireclion))
  (bind _transform (FireAction|CalculateFinalDireclion _location _rotation))
  (Game|SpawnActorfromClass "/Game/Blueprints/BP_Bullet.BP_Bullet_C" _transform "Undefined" 0 0))

(fn CalculateFinalDireclion
  (params (Location :type Vector) (Rotation :type Rotator))
  (bind _weaponspread (Variables|WeaponsSetting|GetWeaponSpread))
  (bind _returnvalue (* _weaponspread -1.0))
  (return (Math|Transform|MakeTransform Location (Math|Rotator|CombineRotators Rotation (Math|Rotator|MakeRotator (Math|Random|RandomFloatinRange _returnvalue 0.0) (Math|Random|RandomFloatinRange _returnvalue 0.0) (Math|Random|RandomFloatinRange _returnvalue 0.0))))))

(fn CameraToggle
  (params (Condition :type Boolean))
  (if Condition
    _))

(fn PlayMontage
  (bind _charactersref (Variables|Default|GetCharactersRef))
  (bind _masterweaponinfo (Variables|Default|GetMasterWeaponInfo))
  (bind _animationsetup (Utilities|Struct|BreakStruct_MasterWeapon _masterweaponinfo))
  (if (Variables|Default|GetAttached?)
    (Animation|Montage|MontagePlay (Components|SkeletalMesh|GetAnimInstance (Variables|Default|GetSkeletalMesh)) (.m_weaponfire _animationsetup) 1.0 "MontageLength" 0.0 true)
    (Animation|Montage|MontagePlay (Components|SkeletalMesh|GetAnimInstance (Variables|/Script/Engine.Character|GetMesh _charactersref)) (select (Variables|/Game/Blueprints/Character/ThirdPersonCharacter.ThirdPersonCharacter_C|GetAiming _charactersref) (.m_character_aimfire _animationsetup) (.m_character_fire _animationsetup)) 1.0 "MontageLength" 0.0 true)))

(fn Reload
  (if (Variables|Default|GetAttached?)
    (if (not (LocalVariables|GetCanFire?))
      (if (> (.AmmoMax (Utilities|Struct|BreakStruct_ShootingSettings (Utilities|Struct|BreakStruct_MasterWeapon (Variables|Default|GetMasterWeaponInfo)))) 0)
        (Variables|WeaponsSetting|SetNededAmmo (- (.AmmoInClip (Utilities|Struct|BreakStruct_ShootingSettings (Utilities|Struct|BreakStruct_MasterWeapon (Variables|Default|GetMasterWeaponInfo)))) (.AmmoCurrent (Utilities|Struct|BreakStruct_ShootingSettings (Utilities|Struct|BreakStruct_MasterWeapon (Variables|Default|GetMasterWeaponInfo))))))
        (if (<= (.AmmoMax (Utilities|Struct|BreakStruct_ShootingSettings (Utilities|Struct|BreakStruct_MasterWeapon (Variables|Default|GetMasterWeaponInfo)))) (Variables|WeaponsSetting|GetNededAmmo))
          (Variables|Default|SetMasterWeaponInfo (Utilities|Struct|MakeStruct_MasterWeapon (.BaseWeaponType (Utilities|Struct|BreakStruct_MasterWeapon (Variables|Default|GetMasterWeaponInfo))) (.DamageSetup (Utilities|Struct|BreakStruct_MasterWeapon (Variables|Default|GetMasterWeaponInfo))) (.SoundEffects (Utilities|Struct|BreakStruct_MasterWeapon (Variables|Default|GetMasterWeaponInfo))) (.VisualEffects (Utilities|Struct|BreakStruct_MasterWeapon (Variables|Default|GetMasterWeaponInfo))) (.AnimationSetup (Utilities|Struct|BreakStruct_MasterWeapon (Variables|Default|GetMasterWeaponInfo))) (Utilities|Struct|MakeStruct_ShootingSettings (.RecoilStrength (Utilities|Struct|BreakStruct_ShootingSettings (.ShootingData (Utilities|Struct|BreakStruct_MasterWeapon (Variables|Default|GetMasterWeaponInfo))))) (.BulletSpeed (Utilities|Struct|BreakStruct_ShootingSettings (.ShootingData (Utilities|Struct|BreakStruct_MasterWeapon (Variables|Default|GetMasterWeaponInfo))))) (.ReloadDelay (Utilities|Struct|BreakStruct_ShootingSettings (.ShootingData (Utilities|Struct|BreakStruct_MasterWeapon (Variables|Default|GetMasterWeaponInfo))))) 0 (+ (.AmmoMax (Utilities|Struct|BreakStruct_ShootingSettings (.ShootingData (Utilities|Struct|BreakStruct_MasterWeapon (Variables|Default|GetMasterWeaponInfo))))) (.AmmoCurrent (Utilities|Struct|BreakStruct_ShootingSettings (.ShootingData (Utilities|Struct|BreakStruct_MasterWeapon (Variables|Default|GetMasterWeaponInfo)))))) (.AmmoInClip (Utilities|Struct|BreakStruct_ShootingSettings (.ShootingData (Utilities|Struct|BreakStruct_MasterWeapon (Variables|Default|GetMasterWeaponInfo))))) (.BulletCountOnSingleShot (Utilities|Struct|BreakStruct_ShootingSettings (.ShootingData (Utilities|Struct|BreakStruct_MasterWeapon (Variables|Default|GetMasterWeaponInfo))))) (.AutoFireCauntDelay (Utilities|Struct|BreakStruct_ShootingSettings (.ShootingData (Utilities|Struct|BreakStruct_MasterWeapon (Variables|Default|GetMasterWeaponInfo))))) (.CanSingleFire (Utilities|Struct|BreakStruct_ShootingSettings (.ShootingData (Utilities|Struct|BreakStruct_MasterWeapon (Variables|Default|GetMasterWeaponInfo))))) (.CanAutoFire (Utilities|Struct|BreakStruct_ShootingSettings (.ShootingData (Utilities|Struct|BreakStruct_MasterWeapon (Variables|Default|GetMasterWeaponInfo))))) (.CameraShakeOnShoot (Utilities|Struct|BreakStruct_ShootingSettings (.ShootingData (Utilities|Struct|BreakStruct_MasterWeapon (Variables|Default|GetMasterWeaponInfo))))))))
          (else
            (Variables|Default|SetMasterWeaponInfo (Utilities|Struct|MakeStruct_MasterWeapon (.BaseWeaponType (Utilities|Struct|BreakStruct_MasterWeapon (Variables|Default|GetMasterWeaponInfo))) (.DamageSetup (Utilities|Struct|BreakStruct_MasterWeapon (Variables|Default|GetMasterWeaponInfo))) (.SoundEffects (Utilities|Struct|BreakStruct_MasterWeapon (Variables|Default|GetMasterWeaponInfo))) (.VisualEffects (Utilities|Struct|BreakStruct_MasterWeapon (Variables|Default|GetMasterWeaponInfo))) (.AnimationSetup (Utilities|Struct|BreakStruct_MasterWeapon (Variables|Default|GetMasterWeaponInfo))) (Utilities|Struct|MakeStruct_ShootingSettings (.RecoilStrength (Utilities|Struct|BreakStruct_ShootingSettings (.ShootingData (Utilities|Struct|BreakStruct_MasterWeapon (Variables|Default|GetMasterWeaponInfo))))) (.BulletSpeed (Utilities|Struct|BreakStruct_ShootingSettings (.ShootingData (Utilities|Struct|BreakStruct_MasterWeapon (Variables|Default|GetMasterWeaponInfo))))) (.ReloadDelay (Utilities|Struct|BreakStruct_ShootingSettings (.ShootingData (Utilities|Struct|BreakStruct_MasterWeapon (Variables|Default|GetMasterWeaponInfo))))) (- (.AmmoMax (Utilities|Struct|BreakStruct_ShootingSettings (.ShootingData (Utilities|Struct|BreakStruct_MasterWeapon (Variables|Default|GetMasterWeaponInfo))))) (Variables|WeaponsSetting|GetNededAmmo)) (.AmmoInClip (Utilities|Struct|BreakStruct_ShootingSettings (.ShootingData (Utilities|Struct|BreakStruct_MasterWeapon (Variables|Default|GetMasterWeaponInfo))))) (.AmmoInClip (Utilities|Struct|BreakStruct_ShootingSettings (.ShootingData (Utilities|Struct|BreakStruct_MasterWeapon (Variables|Default|GetMasterWeaponInfo))))) (.BulletCountOnSingleShot (Utilities|Struct|BreakStruct_ShootingSettings (.ShootingData (Utilities|Struct|BreakStruct_MasterWeapon (Variables|Default|GetMasterWeaponInfo))))) (.AutoFireCauntDelay (Utilities|Struct|BreakStruct_ShootingSettings (.ShootingData (Utilities|Struct|BreakStruct_MasterWeapon (Variables|Default|GetMasterWeaponInfo))))) (.CanSingleFire (Utilities|Struct|BreakStruct_ShootingSettings (.ShootingData (Utilities|Struct|BreakStruct_MasterWeapon (Variables|Default|GetMasterWeaponInfo))))) (.CanAutoFire (Utilities|Struct|BreakStruct_ShootingSettings (.ShootingData (Utilities|Struct|BreakStruct_MasterWeapon (Variables|Default|GetMasterWeaponInfo))))) (.CameraShakeOnShoot (Utilities|Struct|BreakStruct_ShootingSettings (.ShootingData (Utilities|Struct|BreakStruct_MasterWeapon (Variables|Default|GetMasterWeaponInfo))))))))))
        (|AnimMontagePlay)
        (CallFunction|InfoPanelUpdate)))))

(fn InfoPanelUpdate
  (bind _masterweaponinfo (Variables|Default|GetMasterWeaponInfo))
  (bind _shootingdata (Utilities|Struct|BreakStruct_MasterWeapon _masterweaponinfo))
  (bind (_recoilstrength _bulletspeed _reloaddelay _ammomax _ammocurrent) (Utilities|Struct|BreakStruct_ShootingSettings _shootingdata))
  (Default|UpdateInfo (Variables|Default|GetW%20Weapon%20Info) (* _ammocurrent 0.033) _ammocurrent (Utilities|Text|ToText(Integer) _ammomax)))